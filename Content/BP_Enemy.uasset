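; BP_Enemy is an enemy that periodically turns toward the player and fires projectiles.
; BeginPlay starts a looping timer at the CadenciaDisparo interval, calling Shoot to yaw toward the player pawn and spawn a BP_Bala just ahead.
; DispararPatron spawns a given number of actors with yaws evenly spread around a full circle, but nothing here calls it and its spawn class is unset.
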(event `self.ReceiveBeginPlay`
  (bind _returnvalue (`KismetSystemLibrary.K2_SetTimerDelegate` (delegate `Shoot`) (`self.CadenciaDisparo`) true))
  (set `self.Timer Handle` _returnvalue))

(event `Shoot`
  (bind _returnvalue (`GameplayStatics.GetPlayerPawn` 0))
  (bind (_returnvalue_roll _returnvalue_pitch _returnvalue_yaw) (`KismetMathLibrary.BreakRotator` (`KismetMathLibrary.FindLookAtRotation` (`self.K2_GetActorLocation`) (`self.K2_GetActorLocation` _returnvalue))))
  (`/Engine/EditorBlueprintResources/StandardMacros.IsValid` _returnvalue
    (:`Is Valid`
      (`self.K2_SetActorRotation` (`KismetMathLibrary.MakeRotator` 0.0 0.0 _returnvalue_yaw))
      (`|SpawnActorFromClass` "/Game/BP_Bala.BP_Bala_C" (`KismetMathLibrary.MakeTransform` (+ (+ (`self.K2_GetActorLocation`) (* (`self.GetActorForwardVector`) 100.0)) (0.0 0.0 20.0)) (`self.K2_GetActorRotation`)) "AlwaysSpawn" "MultiplyWithRoot" null null))))

(event `DispararPatron`
  (params (`Add Pin` :type Integer))
  (bind (_returnvalue_roll _returnvalue_pitch _returnvalue_yaw) (`KismetMathLibrary.BreakRotator` (`self.K2_GetActorRotation`)))
  (for _index (range `Add Pin`)
    (`|SpawnActorFromClass` "/Game/BP_Bala.BP_Bala_C" (`KismetMathLibrary.MakeTransform` (+ (+ (`self.K2_GetActorLocation`) (* (`self.GetActorForwardVector`) 100.0)) (0.0 0.0 20.0)) (`KismetMathLibrary.MakeRotator` 0.0 0.0 (+ (* _index (/ 360 `Add Pin`)) _returnvalue_yaw))) "AlwaysSpawn" "MultiplyWithRoot" self null)))

(fn `UserConstructionScript`)